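; BP_Mob is an enemy character that perceives the player, attacks with a punch, and can be killed.
; AI perception calls DetectTarget on sighting the player pawn, while losing it starts a clearable 3-second timer before LostTarget runs.
; The Punch component's overlap passes hits to HitAnyDamage, and DoAttackBasic plays the attack montage.
; Taking damage triggers a stun montage and skin change; at zero health it updates the player's kill count and plays death.
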(event `self.ReceiveBeginPlay`)

(event `self.Punch.OnComponentBeginOverlap`
  (params (OverlappedComponent :type "PrimitiveComponent Object Reference") (OtherActor :type "Actor Object Reference") (OtherComp :type "PrimitiveComponent Object Reference") (OtherBodyIndex :type Integer) (bFromSweep :type Boolean) (SweepResult :type "HitResult Structure (by ref)"))
  ;[1 1 1] 데미지
  (`self.HitAnyDamage` OverlappedComponent OtherActor OtherComp OtherBodyIndex bFromSweep SweepResult))

(event `self.AIPerception.OnTargetPerceptionUpdated`
  (params (Actor :type "Actor Object Reference") (Stimulus :type "AIStimulus Structure"))
  ;[1 1 1] 시야/데미지 받을 시 추적 (AI에 인지된 내용을 계속 써야하므로 변수로 승격)
  (if (== Actor (`GameplayStatics.GetPlayerPawn` 0))
    (if (`.bSuccessfullySensed` (break `AIStimulus` Stimulus))
      (`KismetSystemLibrary.K2_ClearAndInvalidateTimerHandle` (`self.TargetLostTimer`)) ; 액터 인지 시 타이머 클리어
      ;[1 1 1] 타깃 인지하는 경우에 대한 동작
      (`self.DetectTarget` Actor)
      (else
        (bind _returnvalue (`KismetSystemLibrary.K2_SetTimerDelegate` (delegate `SetTargetLost`) 3.0)) ; Time 이 흐른 후 Delegate로 받은 SetTargetLost 실행
        (set `self.TargetLostTimer` _returnvalue)))))

(event `SetTargetLost`
  ;[1 1 1] 시야/데미지 받을 시 추적 (AI에 인지된 내용을 계속 써야하므로 변수로 승격)
  ;[1 1 1] 5초 뒤 타깃을 놓친 경우에 대한 동작
  (`self.LostTarget`))

(event `self.ReceiveAnyDamage`
  (params (Damage :type "Float (single-precision)") (DamageType :type "DamageType Object Reference") (InstigatedBy :type "Controller Object Reference") (DamageCauser :type "Actor Object Reference"))
  ;[1 1 1] 데미지
  (bind _returnvalue (`self.GetDamage` Damage))
  (`self.PlayAnimMontage` "/Game/CityofBrass_Enemies/Meshes/Enemy/Corpse/animation/Corpse_Alert_Stunned_Montage.Corpse_Alert_Stunned_Montage" 3.0)
  (`self.SetWhenDamagedSkin` 1 0.5)
  ;;[1 1 1] 죽음
  (if (<= _returnvalue 0.0)
    (set `self.bCanBeDamaged` false)
    (bind _asbp_player_character (cast `/Game/BP/Player/BP_PlayerCharacter` DamageCauser))
    (`/Game/BP/Player/BP_PlayerCharacter.UpdateMobKillCntInfo` _asbp_player_character 1)
    (`self.PlayAnimMontage` "/Game/Asset/Mob/Anim/Corpse_Alert_Death3_Montage.Corpse_Alert_Death3_Montage" 0.5)))

(fn `Do Attack Basic`
  ;[1 1 1] 공격
  (`self.SetIsHittingAndClear` true)
  (`self.PlayAnimMontage` "/Game/Asset/Mob/Anim/Corpse_Alert_Attack_Basic01_Montage.Corpse_Alert_Attack_Basic01_Montage" 0.8))

(fn `UserConstructionScript`)