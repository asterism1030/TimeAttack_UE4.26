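; RPG game mode that respawns the player character whenever it is destroyed.
; On BeginPlay it stores the character's transform and binds a handler to its OnDestroyed event.
; The handler spawns a new BP_PlayerCharacter at the stored transform and has player controller 0 possess it.
; Respawn then reruns the setup on the new pawn, re-saving its transform and rebinding the event so the cycle repeats.
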(event `self.ReceiveBeginPlay`
  (set `self.origin_playerTransform` (`self.GetTransform` (`GameplayStatics.GetPlayerCharacter` 0)) :!label _label)
  (bind _asbp_player_character (cast `/Game/BP/Player/BP_PlayerCharacter` (`GameplayStatics.GetPlayerCharacter` 0)))
  (add `self.OnDestroyed` _asbp_player_character (delegate `spawn`)))

(event `Respawn`
  (goto _label))

(event `spawn` :!signature `self.OnDestroyed`
  (params (DestroyedActor :type "Actor Object Reference"))
  (bind _returnvalue (`|SpawnActorFromClass` "/Game/BP/Player/BP_PlayerCharacter.BP_PlayerCharacter_C" (`self.origin_playerTransform`) "Undefined" "OverrideRootScale" null null))
  (`Controller.Possess` (`GameplayStatics.GetPlayerController` 0) _returnvalue)
  (`self.Respawn`))

(fn `UserConstructionScript`)