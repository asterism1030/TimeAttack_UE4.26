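; BP_PlayerCharacter is the player character, linking health, weapon hits and kill count to the BP_HUD_PlayerView HUD.
; BeginPlay opens the play page, and the first key press starts the countdown timer.
; Weapon overlaps call WeaponDamage; incoming damage runs GetDamage, updates HP display, and a non-positive result plays the death montage, then opens Game Over.
; Helper functions accumulate kills for the HUD and reset HP and kills.
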(event `self.ReceiveBeginPlay`
  ;[1 1 1] HUD 갱신
  (bind _asbp_hud_player_view (cast `/Game/BP/Player/View/BP_HUD_PlayerView` (`PlayerController.GetHUD` (`GameplayStatics.GetPlayerController` 0))))
  (`/Game/BP/Player/View/BP_HUD_PlayerView.Open_Play_Page` _asbp_hud_player_view)
  ;;[1 1 1] 플레이어 정보
  (`/Game/BP/Player/View/BP_UI_Player_View.InitHP` (`/Game/BP/Player/View/BP_HUD_PlayerView.UIView_Play` _asbp_hud_player_view) (`self.full_hp`)))

(event `Key|AnyKey`
  (params (Key :type "Key Structure"))
  ;[1 1 1] 아무 키 입력(플레이 시작)
  (:`Pressed`
    (if (not (`self.isPlayStart`))
      (set `self.isPlayStart` true)
      (bind _asbp_hud_player_view (cast `/Game/BP/Player/View/BP_HUD_PlayerView` (`PlayerController.GetHUD` (`GameplayStatics.GetPlayerController` 0))))
      (`/Game/BP/Player/View/BP_HUD_PlayerView.TimeCountDown` _asbp_hud_player_view null))))

(event `self.weaponCollision.OnComponentBeginOverlap`
  (params (OverlappedComponent :type "PrimitiveComponent Object Reference") (OtherActor :type "Actor Object Reference") (OtherComp :type "PrimitiveComponent Object Reference") (OtherBodyIndex :type Integer) (bFromSweep :type Boolean) (SweepResult :type "HitResult Structure (by ref)"))
  ;[1 1 1] 데미지
  (`self.WeaponDamage` OverlappedComponent OtherActor OtherComp OtherBodyIndex bFromSweep SweepResult))

(event `self.ReceiveAnyDamage`
  (params (Damage :type "Float (single-precision)") (DamageType :type "DamageType Object Reference") (InstigatedBy :type "Controller Object Reference") (DamageCauser :type "Actor Object Reference"))
  ;[1 1 1] 데미지
  (bind _returnvalue (`self.GetDamage` Damage DamageType InstigatedBy DamageCauser))
  ;;[1 1 1] HUD 갱신
  (bind _asbp_hud_player_view (cast `/Game/BP/Player/View/BP_HUD_PlayerView` (`PlayerController.GetHUD` (`GameplayStatics.GetPlayerController` 0))))
  (`/Game/BP/Player/View/BP_UI_Player_View.UpdateHP` (`/Game/BP/Player/View/BP_HUD_PlayerView.UIView_Play` _asbp_hud_player_view) (`self.remain_hp`) (`self.full_hp`))
  (if (<= _returnvalue 0.0)
    (bind _returnvalue_2 (`self.PlayAnimMontage` "/Game/Asset/Player/Greystone/Animations/Death_Montage.Death_Montage" 0.5))
    (set `self.bCanBeDamaged` false)
    (`KismetSystemLibrary.Delay` _returnvalue_2)
    ;;[1 1 1] HUD - Game Over
    (bind _asbp_hud_player_view_2 (cast `/Game/BP/Player/View/BP_HUD_PlayerView` (`PlayerController.GetHUD` (`GameplayStatics.GetPlayerController` 0))))
    (`/Game/BP/Player/View/BP_HUD_PlayerView.Open_GameOver_Page` _asbp_hud_player_view_2)))

(fn `ResetPlayer`
  (set `self.remain_hp` (`self.full_hp`))
  (set `self.mob_kill_cnt` 0))

(fn `UpdateMobKillCntInfo`
  (params (Cnt :type Integer))
  ;[1 1 1] Player 정보 갱신
  (set `self.mob_kill_cnt` (+ Cnt (`self.mob_kill_cnt`)))
  ;[1 1 1] HUD 갱신
  (bind _asbp_hud_player_view (cast `/Game/BP/Player/View/BP_HUD_PlayerView` (`PlayerController.GetHUD` (`GameplayStatics.GetPlayerController` 0))))
  (`/Game/BP/Player/View/BP_UI_Player_View.UpdateMobKillCnt` (`/Game/BP/Player/View/BP_HUD_PlayerView.UIView_Play` _asbp_hud_player_view) (`self.mob_kill_cnt`)))

(fn `UserConstructionScript`)