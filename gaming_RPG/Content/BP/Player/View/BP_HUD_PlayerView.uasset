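; BP_HUD_PlayerView manages the in-game play HUD, the round countdown and the switch to the game over screen.
; OpenPlayPage creates and shows the player view widget, while TimeCountDown starts a looping one-second timer that refreshes its remaining time.
; When time runs out, the timer clears and resets, then OpenGameOverPage swaps in the game over widget with the player's mob kill count and shows the mouse cursor.
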(event `self.ReceiveBeginPlay`)

(event `TimeCountDown`
  (params (TouchedActor :type "Actor Object Reference"))
  ;[1 1 1] 시간 카운트다운
  (bind _returnvalue (`KismetSystemLibrary.K2_SetTimerDelegate` (delegate `UpdateTimeRemain`) 1.0 true)))

(event `UpdateTimeRemain`
  (bind _remaintime (`self.remainTime`))
  ;[1 1 1] 시간 카운트다운
  ;;[1 1 1] HUD - 남은 시간
  (`/Game/BP/Player/View/BP_UI_Player_View.UpdateRemainTime` (`self.UIView_Play`) _remaintime)
  (set `self.remainTime` (- _remaintime 1))
  (if (< (`self.remainTime`) 0)
    (`KismetSystemLibrary.K2_ClearAndInvalidateTimerHandle` (stale `TimeCountDown` _returnvalue))
    (set `self.remainTime` (`self.originRemainTime`))
    ;;[1 1 1] HUD - Game Over
    (`self.Open_GameOver_Page`)))

(fn `Open_GameOver_Page`
  (bind _returnvalue (`GameplayStatics.GetPlayerController` 0))
  (`Widget.RemoveFromParent` (`self.UIView_Play`))
  (bind _returnvalue_2 (`|CreateWidget` "/Game/BP/Widget/BP_GameOver.BP_GameOver_C" _returnvalue))
  (bind _asplayer_character (cast `PlayerCharacter` (`GameplayStatics.GetPlayerCharacter` 0)))
  (`/Game/BP/Widget/BP_GameOver.UpdateMobKillCnt` _returnvalue_2 (`PlayerCharacter.mob_kill_cnt` _asplayer_character))
  (`UserWidget.AddToViewport` _returnvalue_2 0)
  (set `PlayerController.bShowMouseCursor` true _returnvalue))

(fn `Open_Play_Page`
  (bind _returnvalue (`|CreateWidget` "/Game/BP/Player/View/BP_UI_Player_View.BP_UI_Player_View_C" (`GameplayStatics.GetPlayerController` 0)))
  (bind _output_get (set `self.UIView_Play` _returnvalue))
  (`UserWidget.AddToViewport` _output_get 0))

(fn `UserConstructionScript`)